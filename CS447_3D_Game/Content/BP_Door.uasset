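; BP_Door is a key-locked door that slides open when a ThirdPersonCharacter with enough keys enters its Overlap component.
; On overlap it compares the character's NumberOfKeys to RequiredNumberOfKeys and, if sufficient, subtracts the cost and plays the DoorMovement timeline.
; The timeline's Alpha lerps the Door's relative location from zero to TargetLocation.
; No opened state is tracked, so each qualifying overlap charges keys again.
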(event `self.Overlap.OnComponentBeginOverlap`
  (params (OverlappedComponent :type "PrimitiveComponent Object Reference") (OtherActor :type "Actor Object Reference") (OtherComp :type "PrimitiveComponent Object Reference") (OtherBodyIndex :type Integer) (bFromSweep :type Boolean) (SweepResult :type "HitResult Structure (by ref)"))
  (bind _required_number_of_keys (`self.Required Number of Keys`))
  (bind _asthird_person_character (cast `/Game/ThirdPersonBP/Blueprints/ThirdPersonCharacter` OtherActor))
  (bind _numberofkeys (`/Game/ThirdPersonBP/Blueprints/ThirdPersonCharacter.NumberOfKeys` _asthird_person_character))
  (if (>= _numberofkeys _required_number_of_keys)
    (set `/Game/ThirdPersonBP/Blueprints/ThirdPersonCharacter.NumberOfKeys` (- _numberofkeys _required_number_of_keys) _asthird_person_character) ; set #keys = current keys - keys to open door
    (bind (_direction _alpha) (`Timeline|DoorMovement`)
      (:`Update`
        (`SceneComponent.K2_SetRelativeLocation` (`self.Door`) (`KismetMathLibrary.VLerp` (0.0 0.0 0.0) (`self.Target Location`) _alpha) false false)))))

(fn `UserConstructionScript`)